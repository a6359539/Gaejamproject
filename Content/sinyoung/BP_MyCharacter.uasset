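; BP_MyCharacter is a player character that can jump and mimic possession of a nearby bear while F is held.
; Capsule overlaps track the candidate actor and whether possession is allowed.
; Pressing F saves the transform, spawns a half-scale actor, passes it to the bear's Attachactor and switches the camera to it.
; Releasing F restores transform and view, using view-target changes rather than controller possession.
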(event `InputAction|Jump`
  (params (Key :type "Key Structure"))
  (:`Pressed`
    (`self.Jump`)))

(event `self.Capsule.OnComponentBeginOverlap`
  (params (OverlappedComponent :type "PrimitiveComponent Object Reference") (OtherActor :type "Actor Object Reference") (OtherComp :type "PrimitiveComponent Object Reference") (OtherBodyIndex :type Integer) (bFromSweep :type Boolean) (SweepResult :type "HitResult Structure (by ref)"))
  (set `self.otheractor` OtherActor)
  (set `self.빙의가능` true))

(event `self.Capsule.OnComponentEndOverlap`
  (params (OverlappedComponent :type "PrimitiveComponent Object Reference") (OtherActor :type "Actor Object Reference") (OtherComp :type "PrimitiveComponent Object Reference") (OtherBodyIndex :type Integer))
  (set `self.빙의가능` false))

(event `Key|F`
  (params (Key :type "Key Structure"))
  (:`Pressed`
    (if (`self.빙의가능`)
      (set `self.possessing` true)
      (set `self.tempactortransform` (`self.GetTransform`))
      (bind _returnvalue (`|SpawnActorFromClass` "/Game/sinyoung/possessingactor.possessingactor_C" (`KismetMathLibrary.MakeTransform` (0.0 0.0 0.0) (struct) (0.5 0.5 0.5)) "Undefined" "OverrideRootScale" null null))
      (bind _output_get (set `self.possessingactor` _returnvalue))
      (`/Game/sinyoung/bear.attachactor` (cast `/Game/sinyoung/bear` (`self.otheractor`) :!pure true) _output_get)
      (`PlayerController.SetViewTargetWithBlend` (`GameplayStatics.GetPlayerController` 0) _output_get 0.0 "VTBlend_Linear" 0.0 false)))
  (:`Released`
    (set `self.possessing` false)
    (`self.K2_SetActorTransform` (`self.tempactortransform`))
    (`PlayerController.SetViewTargetWithBlend` (`GameplayStatics.GetPlayerController` 0) self 0.0 "VTBlend_Linear" 0.0 false)))

(fn `UserConstructionScript`)