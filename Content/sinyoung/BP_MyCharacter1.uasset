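; Player character Blueprint with a hold-to-possess mechanic for overlapped defalultchar characters, plus jumping.
; Capsule overlap stores the target and toggles the possession-available flag (빙의가능).
; Pressing F spawns an actor, attaches it to the target, blends the view to it and starts crazy mode.
; Releasing F restores transform and view, possesses the target and clears Crazy; P switches to TESTGM's 2D game camera.
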(event `InputAction|Jump`
  (params (Key :type "Key Structure"))
  (:`Pressed`
    (`self.Jump`)))

(event `self.Capsule.OnComponentBeginOverlap`
  (params (OverlappedComponent :type "PrimitiveComponent Object Reference") (OtherActor :type "Actor Object Reference") (OtherComp :type "PrimitiveComponent Object Reference") (OtherBodyIndex :type Integer) (bFromSweep :type Boolean) (SweepResult :type "HitResult Structure (by ref)"))
  (set `self.otheractor` OtherActor)
  (set `self.빙의가능` true)
  (`KismetSystemLibrary.PrintString` "Hello"))

(event `Key|P`
  (params (Key :type "Key Structure"))
  (:`Pressed`
    (bind _astestgm (cast `/Game/sinyoung/TESTGM` (`GameplayStatics.GetGameMode`) :!label _label))
    (`PlayerController.SetViewTargetWithBlend` (`GameplayStatics.GetPlayerController` 0) (`/Game/sinyoung/TESTGM.2dgamecamera` _astestgm) 0.0 "VTBlend_Linear" 0.0 false)))

(event `self.Capsule.OnComponentEndOverlap`
  (params (OverlappedComponent :type "PrimitiveComponent Object Reference") (OtherActor :type "Actor Object Reference") (OtherComp :type "PrimitiveComponent Object Reference") (OtherBodyIndex :type Integer))
  (set `self.빙의가능` false))

(event `Custom Event_0`
  (goto _label))

(event `Key|F`
  (params (Key :type "Key Structure"))
  (bind _asdefalultchar (cast `/Game/sinyoung/defalultchar` (`self.otheractor`) :!pure true))
  (bind _asdefalultchar_2 (cast `/Game/sinyoung/defalultchar` (`self.otheractor`) :!pure true))
  (:`Pressed`
    (if (`self.빙의가능`)
      (set `self.possessing` true)
      (set `self.tempactortransform` (`self.GetTransform`))
      (bind _returnvalue (`|SpawnActorFromClass` "/Game/sinyoung/possessingactor.possessingactor_C" (`KismetMathLibrary.MakeTransform` (0.0 0.0 0.0) (struct) (0.5 0.5 0.5)) "Undefined" "OverrideRootScale" null null))
      (bind _output_get (set `self.possessingactor` _returnvalue))
      (`/Game/sinyoung/defalultchar.attachactor` _asdefalultchar_2 _output_get)
      (`PlayerController.SetViewTargetWithBlend` (`GameplayStatics.GetPlayerController` 0) _output_get 0.0 "VTBlend_Linear" 0.0 false)
      (`/Game/sinyoung/defalultchar.startcrazymode` _asdefalultchar_2)))
  (:`Released`
    (set `self.possessing` false)
    (`self.K2_SetActorTransform` (`self.tempactortransform`))
    (`PlayerController.SetViewTargetWithBlend` (`GameplayStatics.GetPlayerController` 0) self 0.0 "VTBlend_Linear" 0.0 false)
    (`Controller.Possess` (`GameplayStatics.GetPlayerController` 0) _asdefalultchar)
    (set `/Game/sinyoung/defalultchar.crazy?` false _asdefalultchar)))

(fn `UserConstructionScript`)